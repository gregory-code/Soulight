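; BP_Boulder is a rolling boulder hazard that deals lethal-scale damage to the player.
; On BeginPlay it caches the Sphere's forward vector, then after a short delay applies an impulse along it every tick.
; When Sphere1 overlaps a BP_SPlayer, it deals heavy damage with knockback and destroys itself.
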(event OnComponentBeginOverlap(Sphere1)
  (params (OverlappedComponent :type Primitive%20Component%20Object%20Reference) (OtherActor :type Actor%20Object%20Reference) (OtherComp :type Primitive%20Component%20Object%20Reference) (OtherBodyIndex :type Integer) (bFromSweep :type Boolean) (SweepResult :type Hit%20Result%20Structure%20%28by%20ref%29))
  (bind _asbp_splayer (Utilities|Casting|CastToBP_SPlayer OtherActor))
  (Utilities|IsValid _asbp_splayer
    (:Is%20Valid
      (Class|SCharacterBase|CharacterTakeDamage _asbp_splayer 1e+03 0 (Variables|Default|GetKnockback))
      (Actor|DestroyActor))))

(event EventBeginPlay
  (Variables|Default|SetStartFwd (Math|Vector|GetForwardVector (Variables|Default|GetSphere)))
  (Utilities|FlowControl|Delay 0.3)
  (Variables|Default|SetbStartMoving true))

(event Collision|EventActorBeginOverlap
  (params (OtherActor :type Actor%20Object%20Reference)))

(event EventTick
  (params (DeltaSeconds :type Float%20%28single-precision%29))
  (if (Variables|Default|GetbStartMoving)
    (Physics|AddImpulse (Variables|Default|GetSphere) (* (Variables|Default|GetStartFwd) (Variables|Default|GetForce)) "None" false)))

(fn ConstructionScript)