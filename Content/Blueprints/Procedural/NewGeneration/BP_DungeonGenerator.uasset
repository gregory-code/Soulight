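; Procedural dungeon generator that builds a level from random rooms, with room count scaled by game-instance progress.
; Rooms spawn at random open exits, retrying after a delay when their overlap box hits something.
; Once the count is reached, it places an end room, walls off remaining exits and spawns lamps, a writing table and chests from collected spawn points.
; Tick activates the end room's trigger once three lamps are active.
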(event Custom|StartGenerationTimer
  ;[1 1 1] Generation Timer
  (bind _returnvalue (Utilities|Time|SetTimerbyEvent (delegate Custom|GenerationTimer) 0.0 true))
  (Variables|Default|Timers|SetGenTimerHandle _returnvalue))

(event Custom|GenerationTimer
  ;[1 1 1] Generation Timer
  (if (>= (Utilities|Time|GetGameTimeinSeconds) (Variables|Default|Floats|GetMaxTime))
    (Game|OpenLevel(byObjectReference) "/Game/Levels/Anim_Testing.Anim_Testing")))

(event Custom|Spawn%20Lamps
  ;[1 1 1] Spawn Lamps
  (if (Utilities|Array|IsNotEmpty (Variables|Default|Objects|GetLampSpawnpoints))
    (if (> (Variables|Default|Integers|GetCurrentLampCount) 0)
      (bind _output_get (Variables|Default|SetCurrentLampSpawnPoint (.OutItem (Utilities|Array|Random (Variables|Default|Objects|GetLampSpawnpoints)))))
      (Game|SpawnActorfromClass "/Game/Blueprints/Interactables/BP_Lamp.BP_Lamp_C" (Math|Transform|MakeTransform (Transformation|GetWorldLocation _output_get) "0, 0, 0" "1.000000,1.000000,1.000000") "AlwaysSpawn" "MultiplyWithRoot" 0 0)
      (Variables|Default|Integers|SetCurrentLampCount (- (Variables|Default|Integers|GetCurrentLampCount) 1))
      (Utilities|Array|RemoveItem (Variables|Default|Objects|GetLampSpawnpoints) (Variables|Default|GetCurrentLampSpawnPoint))
      (CallFunction|SpawnLamps))))

(event Custom|Spawn%20Writing%20Table
  ;[1 1 1] Spawn Writing Table
  (Game|SpawnActorfromClass "/Game/Blueprints/Interactables/BP_WritingTable.BP_WritingTable_C" (Math|Transform|MakeTransform (Transformation|GetWorldLocation (.OutItem (Utilities|Array|Random (Variables|Default|Objects|GetWritingTableSpawnPoints)))) "0, 0, 0" "1.000000,1.000000,1.000000") "AlwaysSpawn" "MultiplyWithRoot" 0 0))

(event Custom|Spawn%20Chests
  (bind _chestspawnpoints (Variables|Default|Objects|GetChestSpawnPoints))
  ;[1 1 1] Spawn Chests
  (if (Utilities|Array|IsNotEmpty _chestspawnpoints)
    (bind _array_element (Utilities|Array|ForEachLoopwithBreak _chestspawnpoints :!label _label)
      (:LoopBody
        (if (> (Variables|Default|Integers|GetChestCount) 0)
          (Game|SpawnActorfromClass "/Game/Blueprints/Interactables/BP_Chest.BP_Chest_C" (Math|Transform|MakeTransform (Transformation|GetWorldLocation _array_element) "0, 0, 0" "1.000000,1.000000,1.000000") "AlwaysSpawn" "MultiplyWithRoot" 0 0)
          (Utilities|Array|RemoveItem _chestspawnpoints _array_element)
          (Variables|Default|Integers|SetChestCount (- (Variables|Default|Integers|GetChestCount) 1))
          (else
            (goto _label Break)))))))

(event Custom|Print%20Contents
  ;[1 1 1] Debug
  (for _array_element (Variables|Default|Objects|GetLampSpawnpoints)
    (Development|PrintString (Utilities|GetDisplayName _array_element)))
  (Development|PrintString "Finished"))

(event Custom|Begin%20Generation
  ;[1 1 1] Begin Generation
  (Variables|Default|Integers|SetRoomCount (Variables|Default|Integers|GetMaxRoomCount))
  (CallFunction|SpawnStartRoom)
  (CallFunction|SpawnNextRoom))

(event Custom|ResetGeneration
  ;[1 1 1] Reset Generation
  (for _array_element (Variables|Default|Objects|GetGeneratedRooms)
    (Actor|DestroyActor _array_element))
  (Utilities|Array|Clear (Variables|Default|Objects|GetGeneratedRooms))
  (Utilities|Array|Clear (Variables|Default|Objects|GetExitList)))

(event Custom|Check%20For%20Overlap
  (bind _latestroom (Variables|Default|Objects|GetLatestRoom))
  (bind _overlappedlist (Variables|Default|Objects|GetOverlappedList))
  (bind _latestroom_2 (Variables|Default|Objects|GetLatestRoom))
  ;[1 1 1] Check For Overlap
  (CallFunction|AddOverlappingRoomstoList)
  (if (Utilities|Array|IsNotEmpty (Variables|Default|Objects|GetOverlappedList))
    (Utilities|Array|Clear _overlappedlist)
    (Actor|DestroyActor (Variables|Default|Objects|GetLatestRoom))
    (Utilities|FlowControl|Delay 0.1)
    (CallFunction|SpawnNextRoom)
    (else
      (Utilities|Array|Clear _overlappedlist)
      (Variables|Default|Integers|SetRoomCount (- (Variables|Default|Integers|GetRoomCount) 1))
      (Utilities|Array|RemoveItem (Variables|Default|Objects|GetExitList) (Variables|Default|GetSelected%20Exit%20Point))
      (Utilities|Array|AppendArray (Variables|Default|Objects|GetExitList) (Components|GetChildrenComponents (Variables|/Game/Blueprints/Procedural/NewGeneration/MasterRoom.MasterRoom_C|GetExits%20Folder _latestroom_2) false))
      (Utilities|Array|Add (Variables|Default|Objects|GetGeneratedRooms) _latestroom_2)
      (Utilities|Array|AppendArray (Variables|Default|Objects|GetLampSpawnpoints) (Components|GetChildrenComponents (Variables|/Game/Blueprints/Procedural/NewGeneration/MasterRoom.MasterRoom_C|GetLamp%20Spawnpoint%20Folder _latestroom) false))
      (Utilities|Array|AppendArray (Variables|Default|Objects|GetWritingTableSpawnPoints) (Components|GetChildrenComponents (Variables|/Game/Blueprints/Procedural/NewGeneration/MasterRoom.MasterRoom_C|GetWritingTable%20Spawn%20Point%20Folder _latestroom) false))
      (Utilities|Array|AppendArray (Variables|Default|Objects|GetChestSpawnPoints) (Components|GetChildrenComponents (Variables|/Game/Blueprints/Procedural/NewGeneration/MasterRoom.MasterRoom_C|GetChest%20Spawn%20Point%20Folder _latestroom) false))
      (if (> (Variables|Default|Integers|GetRoomCount) 0)
        (Utilities|FlowControl|Delay 0.1)
        (CallFunction|SpawnNextRoom)
        (else
          (CallFunction|SpawnEndRoom)
          (CallFunction|CloseHoles)
          (CallFunction|SpawnLamps)
          (CallFunction|SpawnWritingTable)
          (CallFunction|SpawnChests)
          (Variables|Default|Bools|SetDungeonComplete true)
          (Utilities|Time|ClearandInvalidateTimerbyHandle (Variables|Default|Timers|GetGenTimerHandle)))))))

(event Custom|Close%20Holes
  ;[1 1 1] Close Holes
  (for _array_element (Variables|Default|Objects|GetExitList)
    (Game|SpawnActorfromClass "/Game/Blueprints/Procedural/NewGeneration/End_Wall.End_Wall_C" (Transformation|GetWorldTransform _array_element) "AlwaysSpawn" "MultiplyWithRoot" 0 0)))

(event Custom|Add%20Overlapping%20Rooms%20To%20List
  ;[1 1 1] Add Overlapping Rooms To List
  (Utilities|Array|AppendArray (Variables|Default|Objects|GetOverlappedList) (Class|PrimitiveComponent|GetOverlappingComponents (Variables|/Game/Blueprints/Procedural/NewGeneration/MasterRoom.MasterRoom_C|GetRoom%20Overlap%20Box (Variables|Default|Objects|GetLatestRoom)))))

(event Custom|Spawn%20Next%20Room
  ;[1 1 1] Spawn Next Room
  (Variables|Default|SetSelected%20Exit%20Point (.OutItem (Utilities|Array|Random (Variables|Default|Objects|GetExitList))))
  (bind _returnvalue (Game|SpawnActorfromClass (.OutItem (Utilities|Array|Random (Variables|Default|Classes|GetRoomList))) (Transformation|GetWorldTransform (Variables|Default|GetSelected%20Exit%20Point)) "AlwaysSpawn" "MultiplyWithRoot" 0 0))
  (bind _asmaster_room (Utilities|Casting|CastToMasterRoom _returnvalue))
  (Variables|Default|Objects|SetLatestRoom _asmaster_room)
  (CallFunction|CheckforOverlap)
  (if true
    (Utilities|Array|RemoveItem (Variables|Default|Objects|GetExitList) 0)))

(event Custom|Spawn%20Start%20Room
  ;[1 1 1] Spawn Start Room
  (bind _returnvalue (Game|SpawnActorfromClass "/Game/Blueprints/Procedural/NewGeneration/DungeonRoom_StartRoom.DungeonRoom_StartRoom_C" (Math|Transform|MakeTransform (Transformation|GetWorldLocation (Variables|Default|GetDefaultSceneRoot)) "0, 0, 0" "1.000000,1.000000,1.000000") "AlwaysSpawn" "MultiplyWithRoot" 0 1 0))
  (Utilities|Array|AppendArray (Variables|Default|Objects|GetExitList) (Components|GetChildrenComponents (Variables|/Game/Blueprints/Procedural/NewGeneration/MasterRoom.MasterRoom_C|GetExits%20Folder _returnvalue) false))
  (Utilities|Array|Add (Variables|Default|Objects|GetGeneratedRooms) _returnvalue))

(event Custom|Spawn%20End%20Room
  (bind _exitlist (Variables|Default|Objects|GetExitList))
  ;[1 1 1] Spawn End Room
  (Utilities|Array|Reverse _exitlist)
  (bind _array_element (Utilities|Array|ForEachLoopwithBreak _exitlist :!label _label)
    (:LoopBody
      (bind _returnvalue (Game|SpawnActorfromClass "/Game/Blueprints/Procedural/NewGeneration/DungeonRoom_End.DungeonRoom_End_C" (Transformation|GetWorldTransform _array_element) "AlwaysSpawn" "MultiplyWithRoot" 0 1 0))
      (Variables|Default|Objects|SetLatestRoom _returnvalue)
      (Utilities|Array|RemoveItem (Variables|Default|Objects|GetExitList) _array_element)
      (CallFunction|AddOverlappingRoomstoList)
      (if (Utilities|Array|IsNotEmpty (Variables|Default|Objects|GetOverlappedList))
        (Utilities|Array|Clear (Variables|Default|Objects|GetOverlappedList))
        (Actor|DestroyActor (Variables|Default|Objects|GetLatestRoom))
        (else
          (Variables|Default|Objects|SetEndRoom _returnvalue)
          (goto _label Break))))))

(event EventBeginPlay
  (bind _asbp_soulight_game_mode (Utilities|Casting|CastToBP_SoulightGameMode (Game|GetGameMode)))
  (Variables|Default|Objects|SetAs%20BP%20Soulight%20Game%20Mode _asbp_soulight_game_mode)
  (bind _asbp_sgame_instance (Utilities|Casting|CastToBP_SGameInstance (Game|GetGameInstance)))
  (bind _output_get (Variables|Default|Objects|SetAs%20BP%20SGame%20Instance _asbp_sgame_instance))
  (Variables|Default|Integers|SetMaxRoomCount (* (Variables|Default|Integers|GetMaxRoomCount) (Variables|/Script/Soulight.SGameInstance|GetCurrentProgress _output_get)))
  (Variables|Default|Integers|SetCurrentLampCount 3)
  (CallFunction|BeginGeneration)
  (CallFunction|StartGenerationTimer))

(event EventTick
  (params (DeltaSeconds :type Float%20%28single-precision%29))
  (bind _as_bp_soulight_game_mode (Variables|Default|Objects|GetAs%20BP%20Soulight%20Game%20Mode))
  (if (not (Variables|Default|Bools|GetObjectiveMet))
    (Utilities|IsValid _as_bp_soulight_game_mode
      (:Is%20Valid
        (bind _returnvalue (Class|SoulightGameMode|GetForestObjectiveTracker _as_bp_soulight_game_mode))
        (if (>= (Class|SForestObjectiveActor|GetActiveLamps _returnvalue) 3)
          (bind _asdungeon_room_end (Utilities|Casting|CastToDungeonRoom_End (Variables|Default|Objects|GetEndRoom)))
          (Rendering|SetVisibility (Variables|/Game/Blueprints/Procedural/NewGeneration/DungeonRoom_End.DungeonRoom_End_C|GetEndTrigger _asdungeon_room_end) true false)
          (Default|ActivateOverlap _asdungeon_room_end)
          (Variables|Default|Bools|SetObjectiveMet true))))))

(fn ConstructionScript)