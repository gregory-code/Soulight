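; Custom PCG element that outputs a random subset of points from each point data on the In pin to ChosenPoints.
; It shuffles points with the context's random stream and adds those with index below Min to new point data.
; A clamped Min-Max count is rolled from a randomly reseeded stream but never used.
; The chosen array is not cleared between inputs, so later outputs accumulate earlier picks.
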(fn ExecutewithContext
  (params (InContext :type PCG%20Context%20Structure%20%28by%20ref%29) (Input :type PCG%20Data%20Collection%20Structure%20%28by%20ref%29))
  (bind _fstream (Variables|Default|GetFStream))
  (bind _returnvalue (Data|GetTypedInputsbyPinLabel Input "In" "/Script/PCG.PCGPointData"))
  (for _array_element _returnvalue
    (bind _output_get (LocalVariables|SetInPointData _array_element))
    (bind _output_get_2 (LocalVariables|SetInPoints (SpatialData|GetPoints _output_get)))
    (Math|Random|SetRandomStreamSeed _fstream (Math|Random|RandomIntegerinRange 0 999999))
    (LocalVariables|SetNumOfElementsToKeep (Math|Integer|Clamp(Integer) (Math|Random|RandomIntegerinRangefromStream _fstream (Variables|Default|GetMin) (Variables|Default|GetMax)) 1 (Utilities|Array|Length _output_get_2)))
    (bind _returnvalue_2 (Class|PCGBlueprintElement|GetRandomStream InContext))
    (Utilities|Array|ShuffleFromStream (LocalVariables|GetInPoints) _returnvalue_2)
    (for (_array_element_2 _array_index) (LocalVariables|GetInPoints)
      (Utilities|Array|Add (select (>= _array_index (Variables|Default|GetMin)) 0 (LocalVariables|GetChosenPoints)) _array_element_2))
    (bind _returnvalue_3 (Game|ConstructObjectfromClass "/Script/PCG.PCGPointData"))
    (bind _output_get_3 (LocalVariables|SetChosenPointsData _returnvalue_3))
    (SpatialData|InitializefromData _output_get_3 (LocalVariables|GetInPointData) 0 true true)
    (SpatialData|SetPoints (LocalVariables|GetChosenPointsData) (LocalVariables|GetChosenPoints))
    (Class|PCGDataFunctionLibrary|AddtoCollection (LocalVariables|GetOutputCollection) (LocalVariables|GetChosenPointsData) "ChosenPoints" (Utilities|Array|MakeArray "")))
  (return (LocalVariables|GetOutputCollection)))