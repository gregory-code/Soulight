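; PCG_Forest is an actor Blueprint that re-randomizes procedurally generated content, likely a forest, each time play begins.
; On BeginPlay it finds a PCGVolume in the level and writes a random value to the "Seed" float parameter on its PCG component's graph instance.
; It then cleans up that component locally and forces regeneration.
; Only a single volume is affected, and the generation rules live in the PCG graph.
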(event EventBeginPlay
  (bind _returnvalue (Actor|GetActorOfClass "/Script/PCG.PCGVolume"))
  (Utilities|IsValid _returnvalue
    (:Is%20Valid
      (bind _output_get (Variables|Default|SetPCG%20Comp (Variables|/Script/PCG.PCGVolume|GetPCGComponent _returnvalue)))
      (Utilities|IsValid (Variables|/Script/PCG.PCGComponent|GetGraphInstance _output_get)
        (:Is%20Valid
          (Effects|Components|ParticleSystem|SetFloatParameter (Variables|/Script/PCG.PCGComponent|GetGraphInstance _output_get) "Seed" (Math|Conversions|ToFloat(Integer) (Math|Random|RandomIntegerinRange 0 999999)))
          (Class|PCGComponent|CleanupLocal (Variables|Default|GetPCG%20Comp) false false)
          (Class|PCGComponent|GenerateLocal (Variables|Default|GetPCG%20Comp) true))))))

(event Collision|EventActorBeginOverlap
  (params (OtherActor :type Actor%20Object%20Reference)))

(event EventTick
  (params (DeltaSeconds :type Float%20%28single-precision%29)))

(fn ConstructionScript)