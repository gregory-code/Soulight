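; Behavior Tree task that makes the AI pawn run away from the actor stored in its Player blackboard key.
; It takes the normalized direction from that actor to the pawn, scales it by Distance and uses AIMoveTo to reach that point.
; A finished move reports success and a failed request reports failure.
; Abort calls FinishExecute with success rather than FinishAbort.
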(event EventReceiveAbortAI
  (params (OwnerController :type AI%20Controller%20Object%20Reference) (ControlledPawn :type Pawn%20Object%20Reference))
  (AI|BehaviorTree|FinishExecute true))

(event EventReceiveExecuteAI
  (params (OwnerController :type AI%20Controller%20Object%20Reference) (ControlledPawn :type Pawn%20Object%20Reference))
  (bind _returnvalue (Transformation|GetActorLocation ControlledPawn))
  (AI|AIMoveTo OwnerController (+ _returnvalue (* (Math|Vector|Normalize (- _returnvalue (Transformation|GetActorLocation (AI|BehaviorTree|GetBlackboardValueasActor (Variables|Default|GetPlayer))))) (Variables|Default|GetDistance))) 0 -1.0 "Default" "Default" true false
    (:OnRequestFailed
      (AI|BehaviorTree|FinishExecute false))
    (:OnMoveFinished
      (AI|BehaviorTree|FinishExecute true))))