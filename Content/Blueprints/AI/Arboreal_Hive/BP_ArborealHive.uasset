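; Arboreal Hive actor that periodically spawns BP_Oakbone actors around itself.
; Tick counts CurrentTime down and resets it to MaxTime after each spawn.
; Each spawn point takes a random side and jitter on X and Y, keeping it offset diagonally from the hive, at a fixed world Z.
; Spawning adjusts for collisions but always succeeds, and nothing here caps the number spawned.
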(event EventBeginPlay)

(event Collision|EventActorBeginOverlap
  (params (OtherActor :type Actor%20Object%20Reference)))

(event EventTick
  (params (DeltaSeconds :type Float%20%28single-precision%29))
  (bind _returnvalue (Transformation|GetActorLocation))
  (bind _returnvalue_2 (+ (.x _returnvalue) 5e+01))
  (bind _returnvalue_3 (- (.x _returnvalue) 5e+01))
  (bind _returnvalue_4 (- (.y _returnvalue) 5e+01))
  (bind _returnvalue_5 (+ (.y _returnvalue) 5e+01))
  (bind _returnvalue_6 (Math|Random|RandomFloatinRange _returnvalue_3 _returnvalue_2))
  (bind _returnvalue_7 (Math|Random|RandomFloatinRange _returnvalue_4 _returnvalue_5))
  (Variables|Default|SetCurrentTime (- (Variables|Default|GetCurrentTime) DeltaSeconds))
  (if (<= (Variables|Default|GetCurrentTime) 0.0)
    (if (>= _returnvalue_6 (.x _returnvalue))
      (Variables|Default|SetSpawn%20Location (Math|Vector|MakeVector (+ _returnvalue_6 1e+02) 0.0 25.0))
      (else
        (Variables|Default|SetSpawn%20Location (Math|Vector|MakeVector (- _returnvalue_6 1e+02) 0.0 25.0))))
    (if (>= _returnvalue_7 (.y _returnvalue))
      (Variables|Default|SetSpawn%20Location (Math|Vector|MakeVector (.x (Variables|Default|GetSpawn%20Location)) (+ _returnvalue_7 1e+02) (.z (Variables|Default|GetSpawn%20Location))))
      (else
        (Variables|Default|SetSpawn%20Location (Math|Vector|MakeVector (.x (Variables|Default|GetSpawn%20Location)) (- _returnvalue_7 1e+02) (.z (Variables|Default|GetSpawn%20Location))))))
    (Game|SpawnActorfromClass "/Game/Blueprints/AI/Oakbone/BP_Oakbone.BP_Oakbone_C" (Math|Transform|MakeTransform (Variables|Default|GetSpawn%20Location) "0, 0, 0" "1.000000,1.000000,1.000000") "AdjustIfPossibleButAlwaysSpawn" "MultiplyWithRoot" 0 0)
    (Variables|Default|SetCurrentTime (Variables|Default|GetMaxTime))))

(fn ConstructionScript)