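; Dreadstorm AI enemy that damages and knocks back the player with swipes from either hand.
; Both hand hitboxes share a HitOnce flag to limit repeat hits, cleared when any overlap on either hand ends.
; SetHandHitboxEnabled toggles overlap events on both hands together.
; Transition sets the Transitioning state, hiding the mesh and widget and deactivating the head hurtbox while true.
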(event OnComponentBeginOverlap(RightHandHitbox)
  (params (OverlappedComponent :type Primitive%20Component%20Object%20Reference) (OtherActor :type Actor%20Object%20Reference) (OtherComp :type Primitive%20Component%20Object%20Reference) (OtherBodyIndex :type Integer) (bFromSweep :type Boolean) (SweepResult :type Hit%20Result%20Structure%20%28by%20ref%29))
  (if (not (Variables|Default|GetHitOnce))
    (bind _assplayer (Utilities|Casting|CastToSPlayer OtherActor))
    (Class|SCharacterBase|TakeDamage _assplayer 15.0 self (Variables|Default|GetSwipeAttackKnockback))
    (Variables|Default|SetHitOnce true)))

(event OnComponentBeginOverlap(LeftHandHitbox)
  (params (OverlappedComponent :type Primitive%20Component%20Object%20Reference) (OtherActor :type Actor%20Object%20Reference) (OtherComp :type Primitive%20Component%20Object%20Reference) (OtherBodyIndex :type Integer) (bFromSweep :type Boolean) (SweepResult :type Hit%20Result%20Structure%20%28by%20ref%29))
  (if (not (Variables|Default|GetHitOnce))
    (bind _assplayer (Utilities|Casting|CastToSPlayer OtherActor))
    (Class|SCharacterBase|TakeDamage _assplayer 15.0 self (Variables|Default|GetSwipeAttackKnockback))
    (Variables|Default|SetHitOnce true)))

(event OnComponentEndOverlap(RightHandHitbox)
  (params (OverlappedComponent :type Primitive%20Component%20Object%20Reference) (OtherActor :type Actor%20Object%20Reference) (OtherComp :type Primitive%20Component%20Object%20Reference) (OtherBodyIndex :type Integer))
  (Variables|Default|SetHitOnce false))

(event OnComponentEndOverlap(LeftHandHitbox)
  (params (OverlappedComponent :type Primitive%20Component%20Object%20Reference) (OtherActor :type Actor%20Object%20Reference) (OtherComp :type Primitive%20Component%20Object%20Reference) (OtherBodyIndex :type Integer))
  (Variables|Default|SetHitOnce false))

(fn ConstructionScript)

(fn Transition
  (params (State :type Boolean))
  (bind _returnvalue (not State))
  (Components|Activation|SetActive (Variables|Default|GetHeadHurtbox) _returnvalue false)
  (Rendering|SetVisibility (Variables|Character|GetMesh) _returnvalue false)
  (Rendering|SetVisibility (Variables|Default|GetWidgetComponent) _returnvalue false)
  (Variables|Default|SetbTransitioning State))

(fn SetHandHitboxEnabled
  (params (State :type Boolean))
  (bind _output_get (Variables|/Script/Engine.PrimitiveComponent|SetbGenerateOverlapEvents (Variables|Default|GetRightHandHitbox) State))
  (Variables|/Script/Engine.PrimitiveComponent|SetbGenerateOverlapEvents (Variables|Default|GetLeftHandHitbox) _output_get))