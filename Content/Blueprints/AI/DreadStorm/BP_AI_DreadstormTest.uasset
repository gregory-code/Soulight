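; BP_AI_DreadstormTest is a test AI controller for Dreadstorm that feeds the player to a behavior tree.
; BeginPlay runs the behavior tree and caches player 0's character as BP_SPlayer.
; Every Tick, while that reference is valid, it writes the player's position and actor to the Location and PlayerName blackboard keys, with no perception check.
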(event EventBeginPlay
  (AI|RunBehaviorTree (Variables|Default|GetBehaviorTree))
  (bind _asbp_splayer (Utilities|Casting|CastToBP_SPlayer (Game|GetPlayerCharacter 0)))
  (Variables|Default|SetAs%20BP%20SPlayer _asbp_splayer))

(event EventTick
  (params (DeltaSeconds :type Float%20%28single-precision%29))
  (bind _blackboard (Variables|Default|GetBlackboard))
  (bind _as_bp_splayer (Variables|Default|GetAs%20BP%20SPlayer))
  (Utilities|IsValid _as_bp_splayer
    (:Is%20Valid
      (AI|Components|Blackboard|SetValueasVector _blackboard (Variables|Default|GetLocation) (Transformation|GetActorLocation _as_bp_splayer))
      (AI|Components|Blackboard|SetValueasObject _blackboard (Variables|Default|GetPlayerName) _as_bp_splayer))))

(fn ConstructionScript)