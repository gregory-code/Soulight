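; AI Blueprint for Silentwing that feeds the player's position into its Blackboard.
; On BeginPlay it casts the first player character to BP_SPlayer and caches it.
; Each Tick it compares the player's location with the last known one and, when it differs beyond a small tolerance, stores it and writes it to a vector Blackboard key, with no perception check.
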(event EventBeginPlay
  (bind _asbp_splayer (Utilities|Casting|CastToBP_SPlayer (Game|GetPlayerCharacter 0)))
  (Variables|Default|SetAs%20BP%20SPlayer _asbp_splayer))

(event EventTick
  (params (DeltaSeconds :type Float%20%28single-precision%29))
  (bind _as_bp_splayer (Variables|Default|GetAs%20BP%20SPlayer))
  (bind _returnvalue (Transformation|GetActorLocation _as_bp_splayer))
  (if (not (Utilities|Operators|EqualEqual _returnvalue (Variables|Default|GetLastKnownLocation) 0.1))
    (bind _output_get (Variables|Default|SetLastKnownLocation _returnvalue))
    (AI|Components|Blackboard|SetValueasVector (AI|GetBlackboard 0) (Variables|Default|GetKey%20Name) _output_get)))

(fn ConstructionScript)