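; BP_Silentwing is the Blueprint for the Silentwing AI enemy, handling its presence on the minimap.
; On BeginPlay it caches BP_SGameInstance, then after a short delay InitIcon registers the actor with that instance's minimap at its current location, using GetIcon and GetIconSize.
; StartDeathBlueprintEvent removes it from the minimap when death starts.
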(event Custom|Init%20Icon
  ;[0 0.3283 1] Init Icon
  (bind _newparam (CallFunction|GetIcon))
  (bind _icon_size (CallFunction|GetIconSize))
  (Class|SMinimap|AddtoMinimap (Class|SGameInstance|GetMinimap (Variables|Default|GetAs%20BP%20SGame%20Instance)) self _newparam _icon_size (Transformation|GetActorLocation)))

(event EventBeginPlay
  (bind _asbp_sgame_instance (Utilities|Casting|CastToBP_SGameInstance (Game|GetGameInstance)))
  (Variables|Default|SetAs%20BP%20SGame%20Instance _asbp_sgame_instance)
  (Utilities|FlowControl|Delay 0.2)
  (CallFunction|InitIcon))

(event EventStartDeathBlueprintEvent
  (Class|SMinimap|RemovefromMinimap (Class|SGameInstance|GetMinimap (Variables|Default|GetAs%20BP%20SGame%20Instance)) self))

(fn ConstructionScript)

(fn GetIcon
  (return "/Game/MinimapTextures/Enemy_Icon.Enemy_Icon"))

(fn GetIconSize
  (return "(X=12.000000,Y=12.000000)"))