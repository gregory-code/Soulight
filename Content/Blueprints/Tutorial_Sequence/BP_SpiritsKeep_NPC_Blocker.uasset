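; A tutorial blocker actor in Spirits Keep that keeps the player in place until they have seen both NPCs.
; When the player overlaps its dialogue trigger, the player character speaks a hint to check the other vendor's.
; It caches the game instance on BeginPlay and polls its HasSeenBothNPCs check every Tick, destroying itself once that returns true.
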(event OnComponentBeginOverlap(DialogueTrigger)
  (params (OverlappedComponent :type Primitive%20Component%20Object%20Reference) (OtherActor :type Actor%20Object%20Reference) (OtherComp :type Primitive%20Component%20Object%20Reference) (OtherBodyIndex :type Integer) (bFromSweep :type Boolean) (SweepResult :type Hit%20Result%20Structure%20%28by%20ref%29))
  (bind _asbp_splayer (Utilities|Casting|CastToBP_SPlayer OtherActor))
  (Class|SPlayer|Speak _asbp_splayer "I should check the other vendor's"))

(event EventBeginPlay
  (bind _assgame_instance (Utilities|Casting|CastToSGameInstance (Game|GetGameInstance)))
  (Variables|Default|SetAs%20SGame%20Instance _assgame_instance))

(event EventTick
  (params (DeltaSeconds :type Float%20%28single-precision%29))
  (bind _as_sgame_instance (Variables|Default|GetAs%20SGame%20Instance))
  (Utilities|IsValid _as_sgame_instance
    (:Is%20Valid
      (if (Class|SGameInstance|HasSeenBothNPCs _as_sgame_instance)
        (Actor|DestroyActor)))))

(fn ConstructionScript)