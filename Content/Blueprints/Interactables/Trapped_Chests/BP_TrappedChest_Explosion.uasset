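; Trapped chest interactable that explodes after the player interacts with it and shows an icon on the minimap until destroyed.
; Interaction makes Tick swell both meshes and drive a dynamic decal material's duration parameter from elapsed time.
; After a delay, it activates Niagara and enables an overlap hitbox that damages and knocks back BP_SPlayer once.
; The actor then leaves the minimap and destroys itself.
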(event OnComponentBeginOverlap(HitBox)
  (params (OverlappedComponent :type Primitive%20Component%20Object%20Reference) (OtherActor :type Actor%20Object%20Reference) (OtherComp :type Primitive%20Component%20Object%20Reference) (OtherBodyIndex :type Integer) (bFromSweep :type Boolean) (SweepResult :type Hit%20Result%20Structure%20%28by%20ref%29))
  (bind _asbp_splayer (Utilities|Casting|CastToBP_SPlayer OtherActor))
  (Utilities|IsValid _asbp_splayer
    (:Is%20Valid
      (Class|SCharacterBase|CharacterTakeDamage _asbp_splayer (Variables|Default|GetDamage) 0 (Variables|Default|GetKnockback))
      (Components|DestroyComponent (Variables|Default|GetHitBox)))))

(event Custom|Init%20Icon
  ;[0 0.3283 1] Init Icon
  (bind _newparam (CallFunction|GetIcon))
  (bind _icon_size (CallFunction|GetIconSize))
  (Class|SMinimap|AddtoMinimap (Class|SGameInstance|GetMinimap (Variables|Default|GetAs%20BP%20SGame%20Instance)) self _newparam _icon_size (Transformation|GetActorLocation)))

(event EventTick
  (params (DeltaSeconds :type Float%20%28single-precision%29))
  (bind _returnvalue (* DeltaSeconds 1e+01))
  (bind _staticmesh (Variables|Default|GetStaticMesh))
  (bind _returnvalue_2 (Transformation|GetWorldScale _staticmesh))
  (bind _returnvalue_3 (Math|Vector|Lerp(Vector) _returnvalue_2 "3.000000,3.000000,3.000000" _returnvalue))
  (if (Variables|Default|GetInteracted)
    (Transformation|SetWorldScale3D _staticmesh _returnvalue_3)
    (Transformation|SetWorldScale3D (Variables|Default|GetStaticMesh1) _returnvalue_3)
    (bind _output_get (Variables|Default|SetCurrentLifetime (+ (Variables|Default|GetCurrentLifetime) DeltaSeconds)))
    (Rendering|Material|SetScalarParameterValue (Variables|Default|GetMaterial) "Current Duration" (Math|Float|Clamp(Float) _output_get) :!class /Script/Engine.MaterialInstanceDynamic)))

(event EventOnInteract
  (params (Player :type S%20Player%20Object%20Reference))
  (bind _hitbox (Variables|Default|GetHitBox))
  (Variables|Default|SetInteracted true)
  (Utilities|FlowControl|Delay 1.5)
  (Components|Activation|Activate (Variables|Default|GetNiagara) false)
  (Collision|SetCollisionEnabled _hitbox "QueryOnly")
  (Collision|SetCollisionResponsetoAllChannels _hitbox "ECR_Overlap")
  (Utilities|FlowControl|Delay 1.0)
  (Class|SMinimap|RemovefromMinimap (Class|SGameInstance|GetMinimap (Variables|Default|GetAs%20BP%20SGame%20Instance)) self)
  (Actor|DestroyActor))

(event EventBeginPlay
  (bind _returnvalue (Rendering|Material|CreateDynamicMaterialInstance (Variables|Default|GetDecal) :!class /Script/Engine.DecalComponent))
  (Variables|Default|SetMaterial _returnvalue)
  (bind _asbp_sgame_instance (Utilities|Casting|CastToBP_SGameInstance (Game|GetGameInstance)))
  (Variables|Default|SetAs%20BP%20SGame%20Instance _asbp_sgame_instance)
  (Utilities|FlowControl|Delay 0.1)
  (CallFunction|InitIcon))

(fn ConstructionScript)

(fn GetIcon
  (return "/Game/UISourceIcons/open-chest-box-6673794-5526410.open-chest-box-6673794-5526410"))

(fn GetIconSize
  (return "(X=12.000000,Y=12.000000)"))