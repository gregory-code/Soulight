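; Trapped chest interactable that turns into an enemy when the player interacts with it.
; On BeginPlay it gets the minimap through the game instance and registers itself with a chest icon after a brief delay.
; On interact, after a short delay, it removes its minimap entry, destroys itself and spawns a BP_Oakbone at its location, ignoring collision.
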(event Custom|Init%20Icon
  ;[0 0.3283 1] Init Icon
  (bind _newparam (CallFunction|GetIcon))
  (bind _icon_size (CallFunction|GetIconSize))
  (Class|SMinimap|AddtoMinimap (Class|SGameInstance|GetMinimap (Variables|Default|GetAs%20BP%20SGame%20Instance)) self _newparam _icon_size (Transformation|GetActorLocation)))

(event EventBeginPlay
  (bind _asbp_sgame_instance (Utilities|Casting|CastToBP_SGameInstance (Game|GetGameInstance)))
  (Variables|Default|SetAs%20BP%20SGame%20Instance _asbp_sgame_instance)
  (Utilities|FlowControl|Delay 0.1)
  (CallFunction|InitIcon))

(event EventOnInteract
  (params (Player :type S%20Player%20Object%20Reference))
  (Utilities|FlowControl|Delay 0.2)
  (Class|SMinimap|RemovefromMinimap (Class|SGameInstance|GetMinimap (Variables|Default|GetAs%20BP%20SGame%20Instance)) self)
  (Actor|DestroyActor)
  (Game|SpawnActorfromClass "/Game/Blueprints/AI/Oakbone/BP_Oakbone.BP_Oakbone_C" (Math|Transform|MakeTransform (Transformation|GetActorLocation) "0, 0, 0" "1.000000,1.000000,1.000000") "AlwaysSpawn" "MultiplyWithRoot" 0 0))

(fn ConstructionScript)

(fn GetIcon
  (return "/Game/UISourceIcons/open-chest-box-6673794-5526410.open-chest-box-6673794-5526410"))

(fn GetIconSize
  (return "(X=12.000000,Y=12.000000)"))