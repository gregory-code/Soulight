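; Enemy projectile actor that destroys itself on a short timer started at BeginPlay.
; Tick is empty, and no movement, collision or damage logic appears in its graphs.
; Disconnected, never-run nodes would find and cache BP_FogOfWarVFX, then feed it the projectile's location and write that location to the MPC_OcclusionMask PlayerLocation parameter.
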(event Custom|DestroyTimer
  (Actor|DestroyActor))

(event EventBeginPlay
  (Utilities|Time|SetTimerbyEvent (delegate Custom|DestroyTimer) 3.0))

(event EventTick
  (params (DeltaSeconds :type Float%20%28single-precision%29)))

(fn ConstructionScript)