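; BP_CameraChangeTrigger is a box trigger that changes the player's camera distance on overlap.
; Its collision switches to query-and-probe shortly after BeginPlay, and overlaps cache the BP_SPlayer reference, skipping the cast once valid.
; If toggled on, it passes custom full-health and empty-health camera positions to the player.
; The toggle-gated camera angle function is called too, but has no implementation.
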(event OnComponentBeginOverlap(Box)
  (params (OverlappedComponent :type Primitive%20Component%20Object%20Reference) (OtherActor :type Actor%20Object%20Reference) (OtherComp :type Primitive%20Component%20Object%20Reference) (OtherBodyIndex :type Integer) (bFromSweep :type Boolean) (SweepResult :type Hit%20Result%20Structure%20%28by%20ref%29))
  (Utilities|IsValid (Variables|Default|GetAs%20BP%20SPlayer)
    (:Is%20Valid
      _)
    (:Is%20Not%20Valid
      (bind _asbp_splayer (Utilities|Casting|CastToBP_SPlayer OtherActor))
      (Variables|Default|SetAs%20BP%20SPlayer _asbp_splayer)))
  (CallFunction|ChangeCameraDistance (Variables|Default|GetFull%20Health%20Camera%20Position) (Variables|Default|GetEmpty%20Health%20Camera%20Position))
  (CallFunction|ChangeCameraAngle (Variables|Default|GetNew%20Camera%20Angle)))

(event EventBeginPlay
  (Utilities|FlowControl|Delay 0.2)
  (Collision|SetCollisionEnabled (Variables|Default|GetBox) "QueryAndProbe"))

(fn ConstructionScript)

(fn ChangeCameraDistance
  (params (Full%20Health%20Position :type Vector) (Empty%20Health :type Vector))
  (bind _as_bp_splayer (Variables|Default|GetAs%20BP%20SPlayer))
  (if (Variables|Default|GetChange%20Camera%20Distance%20Toggle)
    (Class|SPlayer|SetUseCustomHealthPosition _as_bp_splayer true)
    (Class|SPlayer|SetFullHealthPosition _as_bp_splayer Full%20Health%20Position)
    (Class|SPlayer|SetEmptyHealthPosition _as_bp_splayer Empty%20Health)))

(fn ChangeCameraAngle
  (params (New%20Rotation :type Rotator))
  (if (Variables|Default|GetChange%20Camera%20Angle%20Toggle)
    _))