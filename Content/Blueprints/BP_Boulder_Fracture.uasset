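; BP_Boulder_Fracture is an actor, apparently the broken boulder debris, that cleans itself up after spawning.
; BeginPlay waits briefly, sets a StartCleanup flag, then destroys the actor after a further delay.
; While the flag is set, Tick lerps the actor's scale toward zero using DeltaSeconds, giving an eased shrink before removal.
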(event EventBeginPlay
  (Utilities|FlowControl|Delay 2.0)
  (Variables|Default|SetStartCleanup true)
  (Utilities|FlowControl|Delay 5.0)
  (Actor|DestroyActor))

(event EventTick
  (params (DeltaSeconds :type Float%20%28single-precision%29))
  (if (Variables|Default|GetStartCleanup)
    (Transformation|SetActorScale3D (Math|Vector|Lerp(Vector) (Transformation|GetActorScale3D) "0, 0, 0" (* DeltaSeconds 2.0)))))

(fn ConstructionScript)